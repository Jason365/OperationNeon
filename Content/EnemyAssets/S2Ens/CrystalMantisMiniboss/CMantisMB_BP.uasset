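; Crystal Mantis miniboss Blueprint that handles melee damage from its two scythes.
; Overlaps on the left and right scythe colliders both route into SlapPlayerCode, which checks for an actor tagged Player.
; A hit takes one point off PlayerHealth in SurvivalGameMode and plays a sound at the impact point.
; The SwipeShot flag gates damage and clears on a hit; nothing here re-arms it.
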(event OnComponentBeginOverlap(LScytheCol)
  (params (OverlappedComponent :type Primitive%20Component%20Object%20Reference) (OtherActor :type Actor%20Object%20Reference) (OtherComp :type Primitive%20Component%20Object%20Reference) (OtherBodyIndex :type Integer) (bFromSweep :type Boolean) (SweepResult :type Hit%20Result%20Structure%20%28by%20ref%29))
  (Utilities|SlapPlayerCode OtherActor OtherActor SweepResult))

(event OnComponentBeginOverlap(RScytheCol)
  (params (OverlappedComponent :type Primitive%20Component%20Object%20Reference) (OtherActor :type Actor%20Object%20Reference) (OtherComp :type Primitive%20Component%20Object%20Reference) (OtherBodyIndex :type Integer) (bFromSweep :type Boolean) (SweepResult :type Hit%20Result%20Structure%20%28by%20ref%29))
  (Utilities|SlapPlayerCode OtherActor OtherActor SweepResult))

(fn ConstructionScript
  (|CallParentFunction))