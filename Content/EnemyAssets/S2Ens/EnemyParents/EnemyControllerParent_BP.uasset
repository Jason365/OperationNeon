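; Base AI controller for enemies in a VR game, providing shared startup, death handling and combat helpers for child controllers.
; BeginPlay finds the PlayerHead, casts its pawn to EnemyParent_BP, applies per-type stats by AITypeIndex, then activates after a random delay.
; While active, Tick calls the overridable EnAiTick; otherwise it stops movement.
; Helpers cover health, task timers, range, aim with optional offset, line of sight and ground normals.
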(event Custom|PostAIInit
  (params (AnimInst :type Anim%20Instance%20Object%20Reference))
  ;[1 1 1] Event called after ai is started up
)

(event Custom|SubEnemyHit
  (params (Damage :type Float%20%28single-precision%29) (Comp :type Actor%20Component%20Object%20Reference)))

(event Custom|EnemyDie
  ;[1 1 1] Event called when health s 0
  (Default|EnDie (Variables|Default|GetOwnPawnRef)))

(event Custom|OnTakeDMG
  ;[1 1 1] On damage Taken
)

(event Custom|EnAiTick
  (params (DeltaSeconds :type Float%20%28single-precision%29)))

(event EventBeginPlay
  (bind _aitypeindex (Variables|Default|GetAITypeIndex))
  ;[1 1 1] Event begin play
  (bind _outactors (Actor|GetAllActorsOfClass "/Game/VirtualRealityBP/Blueprints/PlayerHead.PlayerHead_C" :!label _label))
  (if (== (Utilities|Array|Length _outactors) 0)
    (Utilities|FlowControl|Delay 0.05)
    (bind _outactors_2 (Actor|GetAllActorsOfClass "/Game/VirtualRealityBP/Blueprints/PlayerHead.PlayerHead_C"))
    (Variables|Default|SetPlayerRef (Utilities|Array|Get(acopy) _outactors_2))
    (else
      (Variables|Default|SetPlayerRef (Utilities|Array|Get(acopy) _outactors))))
  (bind _asenemy_parent_bp (Utilities|Casting|CastToEnemyParent_BP (Pawn|GetControlledPawn))
    (:then
      (bind _output_get (Variables|Default|SetOwnPawnRef _asenemy_parent_bp))
      (CallFunction|PostAIInit (Components|SkeletalMesh|GetAnimInstance (Variables|/Script/Engine.Character|GetMesh _output_get)))
      (Default|UpdateColor (Variables|Default|GetOwnPawnRef))
      (Variables|/Game/EnemyAssets/S2Ens/EnemyParents/EnemyParent_BP.EnemyParent_BP_C|SetMaxHealth (Variables|Default|GetOwnPawnRef) (Utilities|Array|Get(acopy) (Variables|/Game/EnemyAssets/S2Ens/EnemyParents/EnemyParent_BP.EnemyParent_BP_C|GetEnHealthIndex (Variables|Default|GetOwnPawnRef)) _aitypeindex))
      (Variables|/Game/EnemyAssets/S2Ens/EnemyParents/EnemyParent_BP.EnemyParent_BP_C|SetHealth (Variables|Default|GetOwnPawnRef) (Utilities|Array|Get(acopy) (Variables|/Game/EnemyAssets/S2Ens/EnemyParents/EnemyParent_BP.EnemyParent_BP_C|GetEnHealthIndex (Variables|Default|GetOwnPawnRef)) _aitypeindex))
      (Transformation|SetActorScale3D (Variables|Default|GetOwnPawnRef) (Math|Vector|MakeVector (Utilities|Array|Get(acopy) (Variables|/Game/EnemyAssets/S2Ens/EnemyParents/EnemyParent_BP.EnemyParent_BP_C|GetEnScaleIndex (Variables|Default|GetOwnPawnRef)) _aitypeindex) (Utilities|Array|Get(acopy) (Variables|/Game/EnemyAssets/S2Ens/EnemyParents/EnemyParent_BP.EnemyParent_BP_C|GetEnScaleIndex (Variables|Default|GetOwnPawnRef)) _aitypeindex) (Utilities|Array|Get(acopy) (Variables|/Game/EnemyAssets/S2Ens/EnemyParents/EnemyParent_BP.EnemyParent_BP_C|GetEnScaleIndex (Variables|Default|GetOwnPawnRef)) _aitypeindex)))
      (Variables|/Game/EnemyAssets/S2Ens/EnemyParents/EnemyParent_BP.EnemyParent_BP_C|SetBaseScore (Variables|Default|GetOwnPawnRef) (Utilities|Array|Get(acopy) (Variables|/Game/EnemyAssets/S2Ens/EnemyParents/EnemyParent_BP.EnemyParent_BP_C|GetEnBaseScoreIndex (Variables|Default|GetOwnPawnRef)) _aitypeindex))
      (Variables|/Script/Engine.CharacterMovementComponent|SetMaxWalkSpeed (Variables|/Script/Engine.Character|GetCharacterMovement (Variables|Default|GetOwnPawnRef)) (Utilities|Array|Get(acopy) (Variables|/Game/EnemyAssets/S2Ens/EnemyParents/EnemyParent_BP.EnemyParent_BP_C|GetEnSpeedIndex (Variables|Default|GetOwnPawnRef)) _aitypeindex))
      (Variables|/Script/Engine.CharacterMovementComponent|SetMaxFlySpeed (Variables|/Script/Engine.Character|GetCharacterMovement (Variables|Default|GetOwnPawnRef)) (Utilities|Array|Get(acopy) (Variables|/Game/EnemyAssets/S2Ens/EnemyParents/EnemyParent_BP.EnemyParent_BP_C|GetEnSpeedIndex (Variables|Default|GetOwnPawnRef)) _aitypeindex))
      (Development|PrintString "Starting up")
      (Utilities|FlowControl|Delay (Math|Random|RandomFloatinRange 0.1 1.0))
      (Variables|Default|SetIsActive true))
    (:CastFailed
      (Development|PrintString "Not EnemyParent")
      (Utilities|FlowControl|Delay 0.2)
      (goto _label))))

(event EventTick
  (params (DeltaSeconds :type Float%20%28single-precision%29))
  (if (Variables|Default|GetIsActive)
    (CallFunction|EnAiTick DeltaSeconds)
    (else
      (Utilities|FreezeMovement))))

(fn ConstructionScript)

(fn CheckHealth
  (if (<= (Variables|/Game/EnemyAssets/S2Ens/EnemyParents/EnemyParent_BP.EnemyParent_BP_C|GetHealth (Variables|Default|GetOwnPawnRef)) 0.0)
    (if (Variables|Default|GetIsActive)
      (CallFunction|EnemyDie)
      (Variables|Default|SetIsActive false)))
  (return))

(fn FindGroundNormalVector
  (params (SelfRef :type Actor%20Object%20Reference))
  (bind _returnvalue (Transformation|GetActorLocation SelfRef))
  (bind _outhit (Collision|LineTraceByChannel (- _returnvalue "0, 0,100.000000") _returnvalue "TraceTypeQuery1" false 0 "None"))
  (Transformation|SetActorRotation SelfRef (Math|Rotator|FindLookatRotation (+ (.ImpactPoint (Collision|BreakHitResult _outhit)) (.ImpactNormal (Collision|BreakHitResult _outhit))) (.ImpactPoint (Collision|BreakHitResult _outhit)))))

(fn FindSocketValues
  (params (InSocketName :type Name))
  (bind _ownpawnref (Variables|Default|GetOwnPawnRef))
  (bind _mesh (Variables|/Script/Engine.Character|GetMesh _ownpawnref))
  (return (Transformation|GetSocketLocation _mesh InSocketName) (Transformation|GetSocketRotation _mesh InSocketName)))

(fn FindFireVector
  (params (Start :type Vector%20%28by%20ref%29) (Magnitude :type Float%20%28single-precision%29) (ShouldOffset :type Boolean) (offsetAmount :type Float%20%28single-precision%29))
  (bind _playerref (Variables|Default|GetPlayerRef))
  (bind _returnvalue (Transformation|GetActorLocation _playerref))
  (bind _returnvalue_2 (Math|Rotator|FindLookatRotation Start _returnvalue))
  (if ShouldOffset
    (bind (_finalrot _forwardv) (CallFunction|SimpleRotOffset offsetAmount _returnvalue_2))
    (return (* _forwardv Magnitude) _finalrot)
    (else
      (return (* (Math|Vector|GetForwardVector _returnvalue_2) Magnitude) _returnvalue_2))))

(fn CheckTaskTime
  (params (DTime :type Float%20%28single-precision%29))
  (Variables|Default|SetTaskTimer (- (Variables|Default|GetTaskTimer) DTime))
  (return (<= (Variables|Default|GetTaskTimer) 0.0)))

(fn CheckTargetRange
  (params (Range :type Float%20%28single-precision%29))
  (return (<= (Math|Vector|VectorLength (- (Transformation|GetActorLocation (Variables|Default|GetPlayerRef)) (Transformation|GetActorLocation (Variables|Default|GetOwnPawnRef)))) Range)))

(fn CheckFireVector
  (params (Start :type Vector))
  (bind _outactors (Actor|GetAllActorsOfClass "/Game/VirtualRealityBP/Blueprints/VRPlayerPawn.VRPlayerPawn_C"))
  (bind _outhit (Collision|LineTraceByChannel Start (Transformation|GetActorLocation (Variables|Default|GetPlayerRef)) "TraceTypeQuery1" false (Utilities|Array|MakeArray (Variables|/Game/VirtualRealityBP/Blueprints/VRPlayerPawn.VRPlayerPawn_C|GetHeadRef (Utilities|Array|Get(acopy) _outactors)) (Variables|/Game/VirtualRealityBP/Blueprints/VRPlayerPawn.VRPlayerPawn_C|GetLeftController (Utilities|Array|Get(acopy) _outactors)) (Variables|/Game/VirtualRealityBP/Blueprints/VRPlayerPawn.VRPlayerPawn_C|GetRightController (Utilities|Array|Get(acopy) _outactors)) (Pawn|GetControlledPawn)) "None"))
  (return (not (.bBlockingHit (Collision|BreakHitResult _outhit)))))

(fn CheckHealthPercent
  (params (Percent :type Float%20%28single-precision%29))
  (bind _ownpawnref (Variables|Default|GetOwnPawnRef))
  (return (> (/ (Variables|/Game/EnemyAssets/S2Ens/EnemyParents/EnemyParent_BP.EnemyParent_BP_C|GetHealth _ownpawnref) (Variables|/Game/EnemyAssets/S2Ens/EnemyParents/EnemyParent_BP.EnemyParent_BP_C|GetMaxHealth _ownpawnref)) Percent)))