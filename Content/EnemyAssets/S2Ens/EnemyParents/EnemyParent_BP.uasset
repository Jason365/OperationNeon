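; Parent Blueprint for enemies that handles damage, scoring and death, awarding points to the SurvivalGameMode once the game has started.
; Damage macros update health and score and show indicators, while hits and no-damage sub-part hits are reported to the EnemyControllerParent_BP.
; A dynamic glow material is colored by the controller's AI type index.
; Death ragdolls the mesh, drops it through world static and destroys it; kill commands zero health and score.
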(event Custom|EnDie
  (bind _scorevalue (Variables|Default|GetScoreValue))
  (bind _mesh (Variables|Character|GetMesh))
  ;[1 1 1] EnemyNaturalDeath
  (bind _assurvival_game_mode (Utilities|Casting|CastToSurvivalGameMode (Game|GetGameMode))
    (:then
      (if (Variables|/Game/VirtualRealityBP/Blueprints/SurvivalGameMode.SurvivalGameMode_C|GetGameStarted _assurvival_game_mode)
        (Variables|/Game/VirtualRealityBP/Blueprints/SurvivalGameMode.SurvivalGameMode_C|SetPlayerScore _assurvival_game_mode (+ (Variables|/Game/VirtualRealityBP/Blueprints/SurvivalGameMode.SurvivalGameMode_C|GetPlayerScore _assurvival_game_mode) _scorevalue))
        (Utilities|ScoreTextPopupCM _scorevalue (+ (Transformation|GetActorLocation) "0, 0,100.000000"))
        (Utilities|KillChargeCM
          (:Out
            _))))
    (:CastFailed
      _))
  (Physics|SetSimulatePhysics _mesh true)
  (Utilities|FlowControl|Delay 3.5)
  (Collision|SetCollisionResponsetoChannel _mesh "ECC_WorldStatic" "ECR_Ignore")
  (Utilities|FlowControl|Delay 0.55)
  (Actor|DestroyActor))

(event Custom|UpdateColor
  (bind _asenemy_controller_parent_bp (Utilities|Casting|CastToEnemyControllerParent_BP (Pawn|GetController)))
  (Rendering|Material|SetVectorParameterValue (Variables|Default|GetDynamicMat1) "Color" (Utilities|Array|Get(acopy) (Variables|Default|GetEnColorIndex) (Variables|/Game/EnemyAssets/S2Ens/EnemyParents/EnemyControllerParent_BP.EnemyControllerParent_BP_C|GetAITypeIndex _asenemy_controller_parent_bp)) :!class /Script/Engine.MaterialInstanceDynamic))

(event Custom|EnKill
  ;[1 1 1] Enemy is told to die via kill command
  (Variables|Default|SetHealth 0.0)
  (Variables|Default|SetScoreValue 0))

(event EventBeginPlay
  (bind _returnvalue (Rendering|Material|CreateDynamicMaterialInstance (Variables|Character|GetMesh) 1 "/Game/EnemyAssets/MaterialsFolder/EnW2GlowMat_Inst.EnW2GlowMat_Inst" "None" :!class /Script/Engine.PrimitiveComponent))
  (Variables|Default|SetDynamicMat1 _returnvalue)
  (bind _asenemy_controller_parent_bp (Utilities|Casting|CastToEnemyControllerParent_BP (Pawn|GetController)))
  (Rendering|Material|SetVectorParameterValue (Variables|Default|GetDynamicMat1) "Color" (Utilities|Array|Get(acopy) (Variables|Default|GetEnColorIndex) (Variables|/Game/EnemyAssets/S2Ens/EnemyParents/EnemyControllerParent_BP.EnemyControllerParent_BP_C|GetAITypeIndex _asenemy_controller_parent_bp)) :!class /Script/Engine.MaterialInstanceDynamic))

(event EventHitNoDamage
  (params (Damage :type Float%20%28single-precision%29) (HitComp :type Actor%20Component%20Object%20Reference))
  ;[1 1 1] Sub Parts damage system
  (bind _asenemy_controller_parent_bp (Utilities|Casting|CastToEnemyControllerParent_BP (Pawn|GetController)))
  (Default|SubEnemyHit _asenemy_controller_parent_bp Damage HitComp))

(event EventDamageBot
  (params (DamageAmount :type Float%20%28single-precision%29) (HitLocation :type Vector :default "0, 0, 0") (HType :type HitType%20Enum :default "NewEnumerator0"))
  (bind (_newhealth _newscore _hp_scalar _hittype) (Utilities|ENTakeDamageCM DamageAmount (Variables|Default|GetHealth) (Variables|Default|GetMaxHealth) (Variables|Default|GetBaseScore) HType)
    (:Out
      (Variables|Default|SetHealth _newhealth)
      (Variables|Default|SetScoreValue _newscore)
      (Utilities|DamageIndPopupCM HitLocation _hittype (Variables|Default|GetDindOffset))
      (bind _asenemy_controller_parent_bp (Utilities|Casting|CastToEnemyControllerParent_BP (Pawn|GetController)))
      (Default|OnTakeDMG _asenemy_controller_parent_bp))))

(event EventCommandKill
  (CallFunction|EnKill))

(fn ConstructionScript)