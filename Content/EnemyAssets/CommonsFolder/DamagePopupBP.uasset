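; Damage popup actor that displays hit feedback through a DamageTextWidget on a widget component.
; On BeginPlay it scales the widget, passes in its hit type, runs the widget's custom start event and rotates once to face the first PlayerHead actor.
; A looping timer then nudges it along local X, so it drifts toward that head's initial position, despite the FloatUpTick name.
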(event Custom|FloatUpTick
  (Transformation|AddActorLocalOffset "0.100000, 0,0.000000" false false))

(event EventBeginPlay
  (bind _returnvalue (Transformation|GetActorLocation))
  (bind _asdamage_text_widget (Utilities|Casting|CastToDamageTextWidget (UserInterface|GetUserWidgetObject (Variables|Default|GetWidget))))
  (Transformation|SetWorldScale3D (Variables|Default|GetWidget) "0.600000,0.600000,0.600000")
  (Variables|/Game/EnemyAssets/CommonsFolder/DamageTextWidget.DamageTextWidget_C|SetHtype _asdamage_text_widget (Variables|Default|GetHitTyp))
  (Variables|Default|SetStartingLocation _returnvalue)
  (bind _outactors (Actor|GetAllActorsOfClass "/Game/VirtualRealityBP/Blueprints/PlayerHead.PlayerHead_C"))
  (Transformation|SetActorRotation (Math|Rotator|FindLookatRotation _returnvalue (Transformation|GetActorLocation (Utilities|Array|Get(acopy) _outactors))))
  (Utilities|Time|SetTimerbyEvent (delegate Custom|FloatUpTick) 0.01 true)
  (Default|CustomStartEv _asdamage_text_widget))

(fn ConstructionScript)