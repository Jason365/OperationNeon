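; Score popup actor that shows points text through a widget component and floats through the world.
; On BeginPlay it caches the widget's score text reference and start location, then rotates once to face the first PlayerHead actor.
; A fast looping timer then nudges it along its local forward and up axes, so it drifts toward that head position while rising.
; The graph neither sets the text nor destroys the actor.
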(event Custom|CustomEvent
  (Transformation|AddActorLocalOffset "0.500000, 0,0.500000" false false))

(event EventBeginPlay
  (bind _returnvalue (Transformation|GetActorLocation))
  (bind _aspoints_text_widget (Utilities|Casting|CastToPointsTextWidget (UserInterface|GetUserWidgetObject (Variables|Default|GetWidget))))
  (Variables|Default|SetScoreTextRef (Variables|/Game/EnemyAssets/CommonsFolder/PointsTextWidget.PointsTextWidget_C|GetScoreText _aspoints_text_widget))
  (Variables|Default|SetStartingLocation _returnvalue)
  (bind _outactors (Actor|GetAllActorsOfClass "/Game/VirtualRealityBP/Blueprints/PlayerHead.PlayerHead_C"))
  (Transformation|SetActorRotation (Math|Rotator|FindLookatRotation _returnvalue (Transformation|GetActorLocation (Utilities|Array|Get(acopy) _outactors))))
  (Utilities|Time|SetTimerbyEvent (delegate Custom|CustomEvent) 0.01 true))

(fn ConstructionScript
  (|CallParentFunction))