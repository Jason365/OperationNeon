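; CGHealthbarBP is an actor that displays the health bar for the Crystal Giant final boss.
; On BeginPlay it gets the bar from its CGHealthbarW widget component, fills it, and finds the first CrystalGiantBossPawn in the level.
; Each Tick it writes the boss's health ratio into the BHP parameter of the bar's dynamic material, and destroys itself once the boss reference is no longer valid.
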(event EventBeginPlay
  (bind _ascghealthbar_w (Utilities|Casting|CastToCGHealthbarW (UserInterface|GetUserWidgetObject (Variables|Default|GetWidget))))
  (Variables|Default|SetHpBarRef (Variables|/Game/EnemyAssets/FinalBosses/CrystalGiant_Boss/CrystalGiant_Assets/CGHealthbarW.CGHealthbarW_C|GetBHealthBar _ascghealthbar_w))
  (bind _returnvalue (Appearance|GetDynamicMaterial (Variables|Default|GetHpBarRef) :!class /Script/UMG.Image))
  (Rendering|Material|SetScalarParameterValue _returnvalue "BHP" 1.0 :!class /Script/Engine.MaterialInstanceDynamic)
  (bind _outactors (Actor|GetAllActorsOfClass "/Game/EnemyAssets/FinalBosses/CrystalGiant_Boss/CrystalGiantBossPawn.CrystalGiantBossPawn_C"))
  (Variables|Default|SetCGRef (Utilities|Array|Get(acopy) _outactors)))

(event EventTick
  (params (DeltaSeconds :type Float%20%28single-precision%29))
  (bind _cgref (Variables|Default|GetCGRef))
  (bind _returnvalue (Appearance|GetDynamicMaterial (Variables|Default|GetHpBarRef) :!class /Script/UMG.Image))
  (Utilities|IsValid _cgref
    (:Is%20Valid
      (Rendering|Material|SetScalarParameterValue _returnvalue "BHP" (/ (Variables|/Game/EnemyAssets/FinalBosses/CrystalGiant_Boss/CrystalGiantBossPawn.CrystalGiantBossPawn_C|GetHealth _cgref) (Variables|/Game/EnemyAssets/FinalBosses/CrystalGiant_Boss/CrystalGiantBossPawn.CrystalGiantBossPawn_C|GetMaxHealth _cgref)) :!class /Script/Engine.MaterialInstanceDynamic))
    (:Is%20Not%20Valid
      (Actor|DestroyActor))))

(fn ConstructionScript)