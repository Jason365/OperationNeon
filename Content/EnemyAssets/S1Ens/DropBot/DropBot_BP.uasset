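; DropBot Blueprint is an enemy bot that can be carried by a CarryBot_Pawn as its child actor and dropped from it.
; The Drop event hands the drop to its DropBotCTRL AI controller.
; On EnDie, a carried bot triggers the carrier's fly-up and calls Drop, and the parent class's death logic also runs.
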(event Custom|Drop
  (bind _asdrop_bot_ctrl (Utilities|Casting|CastToDropBotCTRL (AI|GetAIController self)))
  (Default|DroptheBot _asdrop_bot_ctrl))

(event EventEnDie
  (bind _returnvalue (Actor|GetParentActor))
  (Utilities|IsValid _returnvalue
    (:Is%20Valid
      (bind _ascarry_bot_pawn (Utilities|Casting|CastToCarryBot_Pawn _returnvalue)
        (:then
          (Default|FlyUpTrigger _ascarry_bot_pawn)
          (CallFunction|Drop))
        (:CastFailed
          _)))
    (:Is%20Not%20Valid
      _))
  (|CallParentFunction))

(fn ConstructionScript
  (|CallParentFunction))